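; BP_MobSpawner is a placed actor that spawns a set number of BP_GenericMob instances at its own transform, starting on BeginPlay.
; A DoN node caps the count, and a timer re-fires SpawnNMobs after each spawn to space mobs by a configurable interval.
; SpawnSingleMob creates each mob, sets its GoingTo to the spawner's DestinationPoint and calls OnDestinationChanged on it.
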(event `self.ReceiveBeginPlay`
  (`self.Spawn N Mobs`))

(event `Spawn N Mobs`
  ; Spawns a custom number of mobs at a custom time interval
  (`/Engine/EditorBlueprintResources/StandardMacros.Do N` (`self.NumberOfMobs`)
    (:`Exit`
      (`self.SpawnSingleMob`
        (:`Out`
          (`KismetSystemLibrary.K2_SetTimerDelegate` (delegate `Spawn N Mobs`) (`self.TimeBetweenMobs`)))))))

(fn `UserConstructionScript`)