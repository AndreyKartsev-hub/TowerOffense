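; BP_MobPath is an environment Blueprint that builds a pathway by tiling a mesh along an editable spline, presumably as a route for mobs.
; The construction script derives the tile count from spline length and the mesh's X extent, then adds a collision-enabled spline mesh component per tile.
; A helper function samples local location and tangent at each tile boundary distance to bend each segment along the curve.
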(fn `Get Location and Tangent`
  (params (SplinePointIndex :type Integer))
  (returns (LocationAtDistance :type "Vector Structure") (TangentAtDistance :type "Vector Structure"))
  (bind _spline (`self.Spline`))
  (bind _returnvalue (* SplinePointIndex (`self.MeshLength`)))
  (return (`SplineComponent.GetLocationAtDistanceAlongSpline` _spline _returnvalue "Local") (`SplineComponent.GetTangentAtDistanceAlongSpline` _spline _returnvalue "Local")))

(fn `UserConstructionScript`
  (bind _returnvalue (`StaticMesh.GetBoundingBox` (`self.PathwayMesh`)))
  (set `self.MeshLength` (- (.x (`.Max` (break `Box` _returnvalue))) (.x (break `Box` _returnvalue))))
  ; Iterate through the total number of tiles
  (for _index (range (+ (`KismetMathLibrary.FTrunc` (/ (`SplineComponent.GetSplineLength` (`self.Spline`)) (`self.MeshLength`))) 1))
    (set `self.SplinePointIndex` _index)
    (bind _returnvalue_2 (`AddComponent|NODE_AddSplineMeshComponent-1`))
    ; Tile the spline with a custom mesh
    (`StaticMeshComponent.SetStaticMesh` _returnvalue_2 (`self.PathwayMesh`))
    (`PrimitiveComponent.SetCollisionEnabled` _returnvalue_2 "QueryAndPhysics")
    ; Position and rotate the tiles correctly along the spline
    (bind (_locationatdistance _tangentatdistance) (`self.Get Location and Tangent` (`self.SplinePointIndex`)))
    (bind (_locationatdistance_2 _tangentatdistance_2) (`self.Get Location and Tangent` (+ (`self.SplinePointIndex`) 1)))
    (`SplineMeshComponent.SetStartAndEnd` _returnvalue_2 _locationatdistance _tangentatdistance _locationatdistance_2 _tangentatdistance_2 true)))